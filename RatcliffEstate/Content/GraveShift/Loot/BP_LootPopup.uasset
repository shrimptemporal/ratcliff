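; BP_LootPopup is a floating text actor that shows a loot gain as "+Value", set through SetLootPopupValue.
; Each tick it drifts upward and turns the text to the player controller's rotation, flipped 180 degrees to face the player.
; A dynamic material created at BeginPlay fades the text's Opacity by the ratio of remaining to initial lifespan.
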(event EventBeginPlay
  (bind _returnvalue (Rendering|Material|CreateDynamicMaterialInstance (Variables|Default|GetTextRender) 0 0 "None" :!class /Script/Engine.PrimitiveComponent))
  (Variables|Default|SetDynMat _returnvalue))

(event EventTick
  (params (DeltaSeconds :type Float%20%28single-precision%29))
  (bind _textrender (Variables|Default|GetTextRender))
  (Transformation|SetActorLocation (+ (Transformation|GetActorLocation) (* (Math|Vector|VectorUp) (* DeltaSeconds 1e+02))) false false)
  (Transformation|SetWorldRotation _textrender (.rotation (Transformation|GetActorTransform (Game|GetPlayerController 0))) false false)
  (Transformation|AddLocalRotation _textrender "0.000000,-180.000000,0.000000" false false)
  (Rendering|Material|SetScalarParameterValue (Variables|Default|GetDynMat) "Opacity" (/ (Actor|GetLifeSpan) (Variables|Actor|GetInitialLifeSpan)) :!class /Script/Engine.MaterialInstanceDynamic))

(fn ConstructionScript)

(fn SetLootPopupValue
  (params (Value :type Integer))
  (Rendering|Components|TextRender|SetText (Variables|Default|GetTextRender) (Utilities|Text|ToText(String) (Utilities|String|BuildString(Integer) "" "+" Value))))