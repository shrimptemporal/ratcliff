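; BP_StorageGrave is a grave actor that tells the player's storage component when the player enters or leaves it.
; On begin and end overlap it checks the other actor for the player tag.
; It then calls PlayerInGrave or PlayerLeftGrave on that actor's PlayerStorageComponent, leaving all storage logic to the component.
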(event Collision|EventActorBeginOverlap
  (params (OtherActor :type Actor%20Object%20Reference))
  ;[0.05098 0.05098 0.05098] EVENT ACTOR BEGIN OVERLAP
  (if (Actor|ActorHasTag OtherActor (Variables|Default|GetPlayerTag))
    (Default|PlayerinGrave (Actor|GetComponentbyClass OtherActor "/Game/GraveShift/Player/PlayerStorageComponent.PlayerStorageComponent_C"))))

(event Collision|EventActorEndOverlap
  (params (OtherActor :type Actor%20Object%20Reference))
  ;[0.05098 0.05098 0.05098] EVENT ACTOR END OVERLAP
  (if (Actor|ActorHasTag OtherActor (Variables|Default|GetPlayerTag))
    (Default|PlayerLeftGrave (Actor|GetComponentbyClass OtherActor "/Game/GraveShift/Player/PlayerStorageComponent.PlayerStorageComponent_C"))))

(fn ConstructionScript)