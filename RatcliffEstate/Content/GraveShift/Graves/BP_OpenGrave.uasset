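; Open grave that serves as a player hiding spot in Grave Shift.
; Overlap by a tagged player toggles a text pop-up and allows or disables hiding through the player's PlayerHidingComponent, passing the grave in when allowed.
; CloseDoor and OpenDoor events use separate timelines to lerp the hinge's pitch between open and closed rotations.
; When each animation finishes, the game mode's sound state updates to NO for closed or LOW for open.
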(event Custom|ShowPopUp
  (Rendering|SetVisibility (Variables|Default|GetTextRender) true false))

(event Custom|HidePopUp
  (Rendering|SetVisibility (Variables|Default|GetTextRender) false false))

(event Custom|CloseDoor
  ;[0.05098 0.05098 0.05098] Close Door
  (bind _alpha (Timeline|Timeline PlayFromStart)
    (:Update
      (Transformation|SetRelativeRotation (Variables|Default|GetHinge) (Math|Rotator|MakeRotator 0.0 (Math|Float|Lerp (Variables|Default|GetOpenRotation) (Variables|Default|GetClosedRotation) _alpha) 0.0) false false))
    (:Finished
      (Transformation|SetRelativeRotation (Variables|Default|GetHinge) (Math|Rotator|MakeRotator 0.0 (Variables|Default|GetClosedRotation) 0.0) false false)
      (bind _asbp_grave_shift_game_mode (Utilities|Casting|CastToBP_GraveShift_GameMode (Game|GetGameMode)))
      (Default|UpdateSound _asbp_grave_shift_game_mode "NO"))))

(event Custom|OpenDoor
  ;[0.05098 0.05098 0.05098] Open Door
  (bind _alpha (Timeline|Timeline_0 PlayFromStart)
    (:Update
      (Transformation|SetRelativeRotation (Variables|Default|GetHinge) (Math|Rotator|MakeRotator 0.0 (Math|Float|Lerp (Variables|Default|GetClosedRotation) (Variables|Default|GetOpenRotation) _alpha) 0.0) false false))
    (:Finished
      (Transformation|SetRelativeRotation (Variables|Default|GetHinge) (Math|Rotator|MakeRotator 0.0 (Variables|Default|GetOpenRotation) 0.0) false false)
      (bind _asbp_grave_shift_game_mode (Utilities|Casting|CastToBP_GraveShift_GameMode (Game|GetGameMode)))
      (Default|UpdateSound _asbp_grave_shift_game_mode "LOW"))))

(event EventBeginPlay
  (Rendering|SetVisibility (Variables|Default|GetTextRender) false false))

(event Collision|EventActorBeginOverlap
  (params (OtherActor :type Actor%20Object%20Reference))
  ;[0.05098 0.05098 0.05098] EVENT ACTOR BEGIN OVERLAP
  (if (Actor|ActorHasTag OtherActor (Variables|Default|GetPlayerTag))
    (Default|AllowHiding (Actor|GetComponentbyClass OtherActor "/Game/GraveShift/Player/PlayerHidingComponent.PlayerHidingComponent_C") self)
    (CallFunction|ShowPopUp)))

(event Collision|EventActorEndOverlap
  (params (OtherActor :type Actor%20Object%20Reference))
  ;[0.05098 0.05098 0.05098] EVENT ACTOR END OVERLAP
  (if (Actor|ActorHasTag OtherActor (Variables|Default|GetPlayerTag))
    (Default|DisableHiding (Actor|GetComponentbyClass OtherActor "/Game/GraveShift/Player/PlayerHidingComponent.PlayerHidingComponent_C"))
    (CallFunction|HidePopUp)))

(fn ConstructionScript)