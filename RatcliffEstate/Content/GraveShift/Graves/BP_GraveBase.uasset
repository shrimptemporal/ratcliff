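; Base grave actor that the player digs up to release a burst of random loot.
; Overlap with a tagged player notifies their PlayerDiggingComponent and toggles a progress widget's opacity, showing it only while the grave still has loot.
; Start/StopDigging run or pause a timeline that fills the bar.
; On completion it marks itself empty, launches randomly picked loot with upward-biased impulses, occasionally with a bonus item, and removes its Niagara effect.
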(event Custom|Start%20Digging
  (params (DiggingComponent :type Player%20Digging%20Component%20Object%20Reference))
  ;[0.05098 0.05098 0.05098] Start and Stop Digging
  (bind _time (Timeline|DigTimeline Play)
    (:Update
      (CallFunction|UpdateProgress _time))
    (:Finished
      (Variables|Default|SetIsEmpty true)
      (CallFunction|SpawnLoot)
      (CallFunction|HideProgress)
      (Components|DestroyComponent (Variables|Default|GetNiagara)))))

(event Custom|Stop%20Digging
  ;[0.05098 0.05098 0.05098] Start and Stop Digging
  (bind _time (Timeline|DigTimeline Stop)
    (:Update
      (CallFunction|UpdateProgress _time))
    (:Finished
      (Variables|Default|SetIsEmpty true)
      (CallFunction|SpawnLoot)
      (CallFunction|HideProgress)
      (Components|DestroyComponent (Variables|Default|GetNiagara)))))

(event Custom|Show%20Progress
  (if (not (Variables|Default|GetIsEmpty))
    (bind _asw_grave_progress (Utilities|Casting|CastToW_GraveProgress (UserInterface|GetWidget (Variables|Components|GetProgressBar))))
    (Widget|SetRenderOpacity _asw_grave_progress 1.0)))

(event Custom|Hide%20Progress
  (bind _asw_grave_progress (Utilities|Casting|CastToW_GraveProgress (UserInterface|GetWidget (Variables|Components|GetProgressBar))))
  (Widget|SetRenderOpacity _asw_grave_progress 0.0))

(event Custom|Update%20Progress
  (params (CurrentTime :type Float%20%28double-precision%29))
  (bind _asw_grave_progress (Utilities|Casting|CastToW_GraveProgress (UserInterface|GetWidget (Variables|Components|GetProgressBar))))
  (Progress|SetPercent (Variables|/Game/GraveShift/UI/Widgets/W_GraveProgress.W_GraveProgress_C|GetProgressBar _asw_grave_progress) (/ CurrentTime (Variables|Default|GetTimeToDig))))

(event Custom|Spawn%20Loot
  (bind _returnvalue (Transformation|GetActorTransform))
  (bind _returnvalue_2 (Math|Random|RandomUnitVector))
  (bind _lootcount (Variables|Default|GetLootCount))
  (for _index (range 0 (select (Math|Random|RandomBoolwithWeight 0.1) _lootcount (- _lootcount 1)))
    (bind _returnvalue_3 (Game|SpawnActorfromClass (.OutItem (Utilities|Array|Random (Variables|Default|GetLootObjects))) (Math|Transform|MakeTransform (+ (+ (* (Transformation|GetActorUpVector) 3e+01) (+ (* (Transformation|GetActorForwardVector) 3e+01) (.location _returnvalue))) (* (Math|Random|RandomUnitVector) 1e+02)) (.rotation _returnvalue) "0.500000,0.500000,0.500000") "AdjustIfPossibleButAlwaysSpawn" "MultiplyWithRoot" 0 0))
    (Physics|AddImpulse (Variables|/Script/Engine.StaticMeshActor|GetStaticMeshComponent _returnvalue_3) (* (Math|Vector|Normalize (Math|Vector|MakeVector (.x _returnvalue_2) (.y _returnvalue_2) (Math|Float|Absolute(Float) (.z _returnvalue_2)))) (Variables|Default|GetSpawnExplosionPower)) "None" false)))

(event EventBeginPlay
  (CallFunction|HideProgress))

(event Collision|EventActorBeginOverlap
  (params (OtherActor :type Actor%20Object%20Reference))
  ;[0.05098 0.05098 0.05098] EVENT ACTOR BEGIN OVERLAP
  ; When player begins overlaps with grave, find player digging component and have it update it's PlayerInGrave bool
  (if (Actor|ActorHasTag OtherActor (Variables|Default|GetPlayerTag))
    (Default|PlayerinGrave (Actor|GetComponentbyClass OtherActor "/Game/GraveShift/Player/PlayerDiggingComponent.PlayerDiggingComponent_C") self)
    (CallFunction|ShowProgress)))

(event Collision|EventActorEndOverlap
  (params (OtherActor :type Actor%20Object%20Reference))
  ;[0.05098 0.05098 0.05098] EVENT ACTOR END OVERLAP
  ; When player ends overlap with grave, uncheck bool in digging component
  (if (Actor|ActorHasTag OtherActor (Variables|Default|GetPlayerTag))
    (Default|PlayerLeftGrave (Actor|GetComponentbyClass OtherActor "/Game/GraveShift/Player/PlayerDiggingComponent.PlayerDiggingComponent_C"))
    (CallFunction|HideProgress)))

(fn ConstructionScript)