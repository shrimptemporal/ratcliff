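; Screamer hazard that rises from the ground on spawn and slowly yaws its body to face the player.
; Player overlap triggers a head-tilt scream and reports a loud sound at its location to the player's SoundManager.
; An overlapping Loot-tagged actor is destroyed and soothes it instead, skipping the scream.
; Either outcome disables head overlaps, sinks it via timeline, destroys it and clears its SpawnPoint's spawned flag.
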(event Custom|Passthrough
  (if (not (Variables|Default|GetIsSoothed))
    (Development|PrintString "Scream")
    (bind _asbp_player_character (Utilities|Casting|CastToBP_PlayerCharacter (Game|GetPlayerCharacter 0)))
    (CallFunction|ScreamAnim)
    (Default|PlayLoudSound (Variables|/Game/GraveShift/Soundz/BP_SoundManager.BP_SoundManager_C|GetSoundManager (Variables|/Game/GraveShift/Player/BP_PlayerCharacter.BP_PlayerCharacter_C|GetSoundManager _asbp_player_character)) (Transformation|GetActorLocation) self)
    (CallFunction|Vanish)))

(event Custom|Vanish
  (bind _defaultsceneroot (Variables|Default|GetDefaultSceneRoot))
  (bind _returnvalue (Transformation|GetWorldLocation _defaultsceneroot))
  (Variables|/Script/Engine.PrimitiveComponent|SetbGenerateOverlapEvents (Variables|Default|GetHead) false)
  (bind _alpha (Timeline|Timeline PlayFromStart)
    (:Update
      (Transformation|SetWorldLocation _defaultsceneroot (Math|Vector|MakeVector (.x _returnvalue) (.y _returnvalue) (Math|Float|Lerp 1e+02 -7e+01 _alpha)) false false))
    (:Finished
      (Actor|DestroyActor)
      (Variables|/Game/GraveShift/Screamers/BP_ScreamerSpawnPoint.BP_ScreamerSpawnPoint_C|SetScreamerSpawned (Variables|Default|GetSpawnPoint) false))))

(event Custom|ScreamAnim
  (Audio|PlaySound2D "/Game/Audio/M_Sound/Screamer.Screamer" 1.0 1.0 0.0 0 0)
  (bind _alpha (Timeline|ScreamTimeline PlayFromStart)
    (:Update
      (Transformation|SetRelativeRotation (Variables|Default|GetHeadPivot) (Math|Rotator|MakeRotator (Math|Float|Lerp 0.0 -1.2e+02 _alpha) 0.0 0.0) false false))))

(event Custom|RiseAnim
  (params (EndPoint :type Float%20%28double-precision%29))
  (bind _defaultsceneroot (Variables|Default|GetDefaultSceneRoot))
  (bind _returnvalue (Transformation|GetWorldLocation _defaultsceneroot))
  (bind _newtrack_0 (Timeline|RiseTimeline PlayFromStart)
    (:Update
      (Transformation|SetWorldLocation (Variables|Default|GetDefaultSceneRoot) (Math|Vector|MakeVector (.x _returnvalue) (.y _returnvalue) (Math|Float|Lerp (.z _returnvalue) EndPoint _newtrack_0)) false false))))

(event EventTick
  (params (DeltaSeconds :type Float%20%28single-precision%29))
  (Transformation|SetWorldRotation (Variables|Default|GetBody) (Math|Rotator|MakeRotator 0.0 0.0 (.Yaw (Math|Rotator|BreakRotator (Math|Interpolation|RInterpTo (Transformation|GetWorldRotation (Variables|Default|GetBody)) (Math|Rotator|CombineRotators (Math|Rotator|FindLookatRotation (Transformation|GetWorldLocation (Variables|Default|GetBody)) (Transformation|GetActorLocation (Variables|Default|GetPlayer))) "0.000000,-90.000000,0.000000") DeltaSeconds 1.5)))) false false))

(event Collision|EventActorBeginOverlap
  (params (OtherActor :type Actor%20Object%20Reference))
  (if (Actor|ActorHasTag OtherActor "Player")
    (CallFunction|Passthrough)
    (elif (Actor|ActorHasTag OtherActor "Loot")
      (Variables|Default|SetIsSoothed true)
      (Actor|DestroyActor OtherActor)
      (CallFunction|Vanish))))

(event EventBeginPlay
  (bind _defaultsceneroot (Variables|Default|GetDefaultSceneRoot))
  (bind _returnvalue (Transformation|GetWorldLocation _defaultsceneroot))
  (bind _returnvalue_2 (Actor|GetActorOfClass "/Game/GraveShift/Player/BP_PlayerCharacter.BP_PlayerCharacter_C"))
  (Variables|Default|SetPlayer _returnvalue_2)
  (Transformation|SetWorldLocation (Variables|Default|GetDefaultSceneRoot) (Math|Vector|MakeVector (.x _returnvalue) (.y _returnvalue) (- (.z _returnvalue) 2e+02)) false false)
  (CallFunction|RiseAnim 1e+02))

(fn ConstructionScript)