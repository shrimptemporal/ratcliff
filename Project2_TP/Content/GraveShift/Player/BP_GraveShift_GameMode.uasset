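; Game mode for GraveShift that creates the player HUD and win screen and tracks the player's carried and stored money.
; It caches player component references and relays sound level and eye open/close state to the HUD.
; Money changes update the HUD and the player's weight component, while LootGraph moves money to and from storage or throws it as spawned coin piles.
; Final score sums carried and stored money for the win screen.
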(event Custom|Update%20Money
  (bind _playermoney (Variables|Default|GetPlayerMoney))
  ;[0.05098 0.05098 0.05098] Update Money (updates ui and player weight)
  (Rendering|Components|TextRender|SetText (Variables|/Game/GraveShift/UI/Widgets/W_PlayerUI.W_PlayerUI_C|GetMoneyText (Variables|Default|GetUI%20Widget)) (Utilities|Text|ToText(Integer) _playermoney))
  (Variables|/Game/GraveShift/Player/PlayerWeightComponent.PlayerWeightComponent_C|SetCurrent%20Money (Actor|GetComponentbyClass (Variables|Default|GetPlayer) "/Game/GraveShift/Player/PlayerWeightComponent.PlayerWeightComponent_C") (Math|Conversions|ToFloat(Integer) _playermoney)))

(event Custom|Update%20Sound
  (params (Sound :type Text))
  (bind _returnvalue (Utilities|String|ToString(Text) Sound))
  (bind _ui_widget (Variables|Default|GetUI%20Widget))
  ;[0.05098 0.05098 0.05098] Update Sound (updates ui)
  (Rendering|Components|TextRender|SetText (Variables|/Game/GraveShift/UI/Widgets/W_PlayerUI.W_PlayerUI_C|GetSoundText (Variables|Default|GetUI%20Widget)) "LOW")
  (if (Utilities|Enum|Equal(Enum) _returnvalue "LOW")
    (Default|LowSound _ui_widget)
    (elif (Utilities|Enum|Equal(Enum) _returnvalue "MEDIUM")
      (Default|MediumSound _ui_widget)
      (elif (Utilities|Enum|Equal(Enum) _returnvalue "HIGH")
        (Default|HighSound _ui_widget)))))

(event Custom|Set%20Player%20Ref
  (params (Player :type BP%20Player%20Character%20Object%20Reference))
  ;[0.05098 0.05098 0.05098] Set Player Ref (Gets reference to digging comp, hiding comp, and movement comp)
  (bind _output_get (Variables|Default|SetPlayer Player))
  (Variables|Default|SetDigging%20Component (Variables|/Game/GraveShift/Player/BP_PlayerCharacter.BP_PlayerCharacter_C|GetPlayerDiggingComponent _output_get))
  (Variables|Default|SetHiding%20Component (Variables|/Game/GraveShift/Player/BP_PlayerCharacter.BP_PlayerCharacter_C|GetPlayerHidingComponent _output_get))
  (Variables|Default|SetMovement%20Component (Variables|/Game/GraveShift/Player/BP_PlayerCharacter.BP_PlayerCharacter_C|GetPlayerMovementComponent _output_get)))

(event Custom|Add%20To%20Money
  (params (Money :type Integer))
  ;[0.05098 0.05098 0.05098] Add To Money (adds to local variable then calls update for ui)
  (Variables|Default|SetPlayerMoney (+ Money (Variables|Default|GetPlayerMoney)))
  (CallFunction|UpdateMoney))

(event Custom|EyeOpen
  ;[0.05098 0.05098 0.05098] Eye Open (updates ui)
  (Default|EyeOpen (Variables|Default|GetUI%20Widget))
  (Variables|Default|SetIsEyeOpen true))

(event Custom|EyeClose
  ;[0.05098 0.05098 0.05098] Eye Close (updates ui)
  (Default|EyeClose (Variables|Default|GetUI%20Widget))
  (Variables|Default|SetIsEyeOpen false))

(event Custom|Final%20Score
  ;[0.05098 0.05098 0.05098] Final Score
  (Default|ScoreEvent (Variables|Default|GetWin%20Screen) (+ (Variables|Default|GetMoneyStored) (Variables|Default|GetPlayerMoney))))

(event EventBeginPlay
  ;[0.05098 0.05098 0.05098] Event BeginPlay (Creates UI and adds to viewport)
  (bind _returnvalue (UserInterface|CreateWidget "/Game/GraveShift/UI/Widgets/W_PlayerUI.W_PlayerUI_C"))
  (bind _output_get (Variables|Default|SetUI%20Widget _returnvalue))
  (UserInterface|Viewport|AddtoViewport _output_get 0)
  (bind _returnvalue_2 (UserInterface|CreateWidget "/Game/GraveShift/UI/Widgets/W_WinScreen.W_WinScreen_C"))
  (bind _output_get_2 (Variables|Default|SetWin%20Screen _returnvalue_2))
  (UserInterface|Viewport|AddtoViewport _output_get_2 0))

(event Custom|Throw%20Loot
  (bind _player (Variables|Default|GetPlayer))
  (bind _returnvalue (Transformation|GetActorTransform _player))
  ;[0.05098 0.05098 0.05098] Throw Loot
  (if (>= (Variables|Default|GetPlayerMoney) 25)
    (bind _returnvalue_2 (Game|SpawnActorfromClass "/Game/GraveShift/Loot/BP_LootSilverCoinPile.BP_LootSilverCoinPile_C" (Math|Transform|MakeTransform (+ (* (Transformation|GetActorForwardVector _player) 1.2e+02) (.location _returnvalue)) (.rotation _returnvalue) "0.500000,0.500000,0.500000") "AdjustIfPossibleButAlwaysSpawn" "MultiplyWithRoot" 0 0))
    (CallFunction|AddtoMoney -25)
    (Default|ThrowSelf _returnvalue_2 (Variables|/Game/GraveShift/Player/BP_PlayerCharacter.BP_PlayerCharacter_C|GetSoundManager (Variables|Default|GetPlayer)))))

(event Custom|Store%20Money
  ;[0.05098 0.05098 0.05098] Store Money
  (if (> (Variables|Default|GetPlayerMoney) 0)
    (if (>= (Variables|Default|GetPlayerMoney) (Variables|LootHandling|GetAmountToStore))
      (Variables|Default|SetMoneyStored (+ (Variables|Default|GetMoneyStored) (Variables|LootHandling|GetAmountToStore)))
      (Variables|Default|SetPlayerMoney (- (Variables|Default|GetPlayerMoney) (Variables|LootHandling|GetAmountToStore)))
      (else
        (Variables|Default|SetMoneyStored (+ (Variables|Default|GetMoneyStored) (Variables|Default|GetPlayerMoney)))
        (Variables|Default|SetPlayerMoney 0)))
    (CallFunction|UpdateMoney)))

(event Custom|UnStore%20Money
  ;[0.05098 0.05098 0.05098] Unstore Money
  (if (> (Variables|Default|GetMoneyStored) 0)
    (if (>= (Variables|Default|GetMoneyStored) (Variables|LootHandling|GetAmountToStore))
      (Variables|Default|SetMoneyStored (- (Variables|Default|GetMoneyStored) (Variables|LootHandling|GetAmountToStore)))
      (Variables|Default|SetPlayerMoney (+ (Variables|Default|GetPlayerMoney) (Variables|LootHandling|GetAmountToStore)))
      (else
        (Variables|Default|SetMoneyStored 0)
        (Variables|Default|SetPlayerMoney (+ (Variables|Default|GetMoneyStored) (Variables|Default|GetPlayerMoney)))))
    (CallFunction|UpdateMoney)))

(fn ConstructionScript)