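; BP_Enemy is an AI enemy character that ends the run by opening the death level when it catches the player.
; Each tick it reads the line-of-sight flag from its Blackboard and checks player distance against a kill threshold.
; It exposes functions to set walk speed and to recolor its four eye lights for chasing, searching or patrol states, with sight taking priority over searching.
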(event EventTick
  (params (DeltaSeconds :type Float%20%28single-precision%29))
  (if (and (ScalableFloat|GetValueasBool (AI|GetBlackboard (Components|GetOwner)) (Variables|Default|GetHasLineOfSight)) (< (Transformation|GetDistanceTo (Variables|Default|GetPlayer)) (Variables|Default|GetKillDistance)))
    (Development|PrintString "KILL TIME!")
    (Game|OpenLevel(byObjectReference) (Variables|Default|GetDeathLevel))))

(fn ConstructionScript)

(fn UpdateWalkSpeed
  (params (NewWalkSpeed :type Float%20%28double-precision%29))
  (Variables|/Script/Engine.CharacterMovementComponent|SetMaxWalkSpeed (Variables|Character|GetCharacterMovement) NewWalkSpeed))

(fn UpdateEyeColor
  (params (HasSightLine :type Boolean) (IsSearching :type Boolean))
  (bind _patrolcolor (Variables|Eyes|GetPatrolColor))
  (bind _patrolcolorsmall (Variables|Eyes|GetPatrolColorSmall))
  (bind _alertcolor (Variables|Eyes|GetAlertColor))
  (bind _chasingcolor (Variables|Eyes|GetChasingColor))
  (bind _alertcolorsmall (Variables|Eyes|GetAlertColorSmall))
  (bind _chasingcolorsmall (Variables|Eyes|GetChasingColorSmall))
  (if HasSightLine
    (Rendering|Components|Light|SetLightColor (Variables|Default|GetEyeLightR) _chasingcolor true)
    (Rendering|Components|Light|SetLightColor (Variables|Default|GetEyeLightL) _chasingcolor true)
    (Rendering|Components|Light|SetLightColor (Variables|Default|GetEyeLightSmallR) _chasingcolorsmall true)
    (Rendering|Components|Light|SetLightColor (Variables|Default|GetEyeLightSmallL) _chasingcolorsmall true)
    (elif IsSearching
      (Rendering|Components|Light|SetLightColor (Variables|Default|GetEyeLightR) _alertcolor true)
      (Rendering|Components|Light|SetLightColor (Variables|Default|GetEyeLightL) _alertcolor true)
      (Rendering|Components|Light|SetLightColor (Variables|Default|GetEyeLightSmallR) _alertcolorsmall true)
      (Rendering|Components|Light|SetLightColor (Variables|Default|GetEyeLightSmallL) _alertcolorsmall true)
      (else
        (Rendering|Components|Light|SetLightColor (Variables|Default|GetEyeLightR) _patrolcolor true)
        (Rendering|Components|Light|SetLightColor (Variables|Default|GetEyeLightL) _patrolcolor true)
        (Rendering|Components|Light|SetLightColor (Variables|Default|GetEyeLightSmallR) _patrolcolorsmall true)
        (Rendering|Components|Light|SetLightColor (Variables|Default|GetEyeLightSmallL) _patrolcolorsmall true)))))