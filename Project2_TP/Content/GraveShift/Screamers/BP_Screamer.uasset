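; BP_Screamer is a spawned hazard that turns to face the player and screams when the player overlaps it.
; The scream swings its head pivot and plays a hearable sound through the player's SoundManager.
; An overlapping Loot actor is destroyed and soothes it, preventing the scream.
; Either outcome makes it shrink away on a timeline, destroy itself and clear its SpawnPoint's spawned flag.
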(event Custom|Passthrough
  (if (not (Variables|Default|GetIsSoothed))
    (Development|PrintString "Scream")
    (bind _asbp_player_character (Utilities|Casting|CastToBP_PlayerCharacter (Game|GetPlayerCharacter 0)))
    (CallFunction|ScreamAnim)
    (Default|PlayHearableSound (Variables|/Game/GraveShift/Soundz/BP_SoundManager.BP_SoundManager_C|GetSoundManager (Variables|/Game/GraveShift/Player/BP_PlayerCharacter.BP_PlayerCharacter_C|GetSoundManager _asbp_player_character)) (Transformation|GetActorLocation) self)
    (CallFunction|Vanish)))

(event Custom|Vanish
  (Variables|/Script/Engine.PrimitiveComponent|SetbGenerateOverlapEvents (Variables|Default|GetHead) false)
  (bind _alpha (Timeline|Timeline PlayFromStart)
    (:Update
      (Transformation|SetActorRelativeScale3D (Math|Conversions|ToVector(Float) (Math|Float|Lerp 1.0 0.0 _alpha))))
    (:Finished
      (Actor|DestroyActor)
      (Variables|/Game/GraveShift/Screamers/BP_ScreamerSpawnPoint.BP_ScreamerSpawnPoint_C|SetScreamerSpawned (Variables|Default|GetSpawnPoint) false))))

(event Custom|ScreamAnim
  (bind _alpha (Timeline|ScreamTimeline PlayFromStart)
    (:Update
      (Transformation|SetRelativeRotation (Variables|Default|GetHeadPivot) (Math|Rotator|MakeRotator (Math|Float|Lerp 0.0 -1.2e+02 _alpha) 0.0 0.0) false false))))

(event EventTick
  (params (DeltaSeconds :type Float%20%28single-precision%29))
  (Transformation|SetWorldRotation (Variables|Default|GetBody) (Math|Rotator|MakeRotator 0.0 0.0 (.Yaw (Math|Rotator|BreakRotator (Math|Interpolation|RInterpTo (Transformation|GetWorldRotation (Variables|Default|GetBody)) (Math|Rotator|CombineRotators (Math|Rotator|FindLookatRotation (Transformation|GetWorldLocation (Variables|Default|GetBody)) (Transformation|GetActorLocation (Variables|Default|GetPlayer))) "0.000000,-90.000000,0.000000") DeltaSeconds 1.5)))) false false))

(event Collision|EventActorBeginOverlap
  (params (OtherActor :type Actor%20Object%20Reference))
  (if (Actor|ActorHasTag OtherActor "Player")
    (CallFunction|Passthrough)
    (elif (Actor|ActorHasTag OtherActor "Loot")
      (Variables|Default|SetIsSoothed true)
      (Actor|DestroyActor OtherActor)
      (CallFunction|Vanish))))

(event EventBeginPlay
  (bind _returnvalue (Actor|GetActorOfClass "/Game/GraveShift/Player/BP_PlayerCharacter.BP_PlayerCharacter_C"))
  (Variables|Default|SetPlayer _returnvalue))

(fn ConstructionScript)