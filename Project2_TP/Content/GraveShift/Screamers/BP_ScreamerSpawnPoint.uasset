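; BP_ScreamerSpawnPoint is a placed spawn point that creates a single screamer enemy at its own location.
; SpawnScreamer runs only while ScreamerSpawned is false, picking BP_HorizontalScreamer or BP_Screamer based on the SpawnHorizontal flag.
; It hands itself to the spawned screamer as SpawnPoint, then sets the flag so further calls spawn nothing.
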(fn ConstructionScript)

(fn SpawnScreamer
  (bind _returnvalue (Transformation|GetActorLocation))
  (bind _self self)
  (bind _returnvalue_2 (Math|Conversions|ToTransform(Vector) _returnvalue))
  (if (not (Variables|Default|GetScreamerSpawned))
    (if (Variables|Default|GetSpawnHorizontal)
      (bind _returnvalue_3 (Game|SpawnActorfromClass "/Game/GraveShift/Screamers/BP_HorizontalScreamer.BP_HorizontalScreamer_C" _returnvalue_2 "Undefined" "MultiplyWithRoot" 0 0))
      (Variables|/Game/GraveShift/Screamers/BP_Screamer.BP_Screamer_C|SetSpawnPoint _returnvalue_3 _self)
      (else
        (bind _returnvalue_4 (Game|SpawnActorfromClass "/Game/GraveShift/Screamers/BP_Screamer.BP_Screamer_C" _returnvalue_2 "Undefined" "MultiplyWithRoot" 0 0))
        (Variables|/Game/GraveShift/Screamers/BP_Screamer.BP_Screamer_C|SetSpawnPoint _returnvalue_4 _self)))
    (Variables|Default|SetScreamerSpawned true)))