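; BP_LootObject is a money pickup that the player collects automatically by coming close to it.
; BeginPlay caches the player by tag, then Tick checks distance and, in range, adds Value to the player's PlayerDiggingComponent.
; Collection also plays a sound, destroys the actor and spawns a BP_LootPopup showing the value.
; SetValue sets the worth, and ThrowSelf stores a sound manager, flags InAir and launches the mesh forward and upward with a physics impulse.
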(event Custom|Set%20Value
  (params (NewValue :type Integer))
  (Variables|Default|SetValue NewValue))

(event Custom|ThrowSelf
  (params (SoundManager :type BP%20Sound%20Manager%20Object%20Reference))
  (Variables|Default|SetSoundManagerRef SoundManager)
  (Variables|Default|SetInAir true)
  (Physics|AddImpulse (Variables|Debug|GetStaticMeshComponent) (+ (* (Transformation|GetActorForwardVector) 5e+03) (* (Transformation|GetActorUpVector) 2e+03)) "None" false))

(event EventTick
  (params (DeltaSeconds :type Float%20%28single-precision%29))
  (bind _player (Variables|Default|GetPlayer))
  (if (< (Transformation|GetDistanceTo _player) (Variables|Default|GetCollectDistance))
    ;[0.01938 0.01938 0.01938] Gets picked up by player
    (Default|AddMoney (Actor|GetComponentbyClass _player "/Game/GraveShift/Player/PlayerDiggingComponent.PlayerDiggingComponent_C") (Variables|Default|GetValue))
    (Audio|PlaySound2D "/Game/Audio/SFX/LootBig.LootBig" 1.0 1.0 0.0 0 0)
    (Actor|DestroyActor)
    (bind _returnvalue (Game|SpawnActorfromClass "/Game/GraveShift/Loot/BP_LootPopup.BP_LootPopup_C" (Transformation|GetActorTransform) "Undefined" "MultiplyWithRoot" 0 0))
    (Default|SetLootPopupValue _returnvalue (Variables|Default|GetValue))))

(event EventBeginPlay
  (bind _outactors (Actor|GetAllActorswithTag (Variables|Default|GetPlayerTag)))
  (bind _asbp_player_character (Utilities|Casting|CastToBP_PlayerCharacter (Utilities|Array|Get(acopy) _outactors))
    (:then
      (Variables|Default|SetPlayer _asbp_player_character))
    (:CastFailed
      (Development|PrintString "Couldn't find a player!"))))

(fn ConstructionScript)